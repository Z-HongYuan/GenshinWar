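; Player camera manager that drives a third/first-person camera for targets tagged NeedCamera, falling back to default behavior otherwise.
; On possess it hands pawn and controller to the CameraMesh's ABP_Camera, whose animation curves supply lag speeds, offsets and first-person weight.
; Pawn interface calls provide targets, FOVs and trace settings for smoothing the pivot per axis in camera-yaw space.
; A sphere trace emulates a spring arm before blending toward first person.
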(event Custom|OnPossess
  (params (ControlledPawn :type Pawn%20Object%20Reference))
  (Variables|Default|SetControlledPawn ControlledPawn)
  (bind _asabp_camera (Utilities|Casting|CastToABP_Camera (Components|SkeletalMesh|GetAnimInstance (Variables|Default|GetCameraMesh))))
  (Variables|/Game/Blueprints/CameraSystem/ABP_Camera.ABP_Camera_C|SetControlledPawn _asabp_camera (Variables|Default|GetControlledPawn))
  (Variables|/Game/Blueprints/CameraSystem/ABP_Camera.ABP_Camera_C|SetPlayerController _asabp_camera (Game|Player|GetOwningPlayerController))
  (Default|OnPossess _asabp_camera))

(fn ConstructionScript)

(fn BlueprintUpdateCamera
  (params (CameraTarget :type Actor%20Object%20Reference))
  (if (Actor|ActorHasTag CameraTarget "NeedCamera")
    (bind (_location _rotation _fov) (ToolFunction|CalculateCameraParameters))
    (return _location _rotation _fov true)
    (else
      (bind (_newcameralocation _newcamerarotation _newcamerafov _returnvalue) (|CallParentFunction 0))
      (return _newcameralocation _newcamerarotation _newcamerafov _returnvalue))))

(fn CalculateCameraParameters
  (bind _returnvalue (ToolFunction|GetCurveValues "Weight_FirstPerson"))
  (Utilities|FlowControl|Sequence
    (:then_0
      ;[0.15 0.15 0.15 0.5] 从Pawn获取Info
      (bind _returnvalue_2 (Class|BPICameraInfo|BPIGet3PPivotTarget(Message) (Variables|Default|GetControlledPawn)))
      (LocalVariables|SetPivotTarget _returnvalue_2)
      (bind _returnvalue_3 (Class|BPICameraInfo|BPIGetFPCameraTarget(Message) (Variables|Default|GetControlledPawn)))
      (LocalVariables|SetFPTarget _returnvalue_3)
      (bind (_tp_fov _fp_fov) (Class|BPICameraInfo|BPIGetCameraParameters(Message) (Variables|Default|GetControlledPawn)))
      (LocalVariables|SetTPFOV _tp_fov)
      (LocalVariables|SetFPFOV _fp_fov))
    (:then_1
      ;[0.15 0.15 0.15 0.5] Smooth Camera Rotation
      (Variables|CameraInfo|SetTargetCameraRotation (Math|Interpolation|RInterpTo (Camera|GetCameraRotation) (Pawn|GetControlRotation (Game|Player|GetOwningPlayerController) :!class /Script/Engine.Controller) (Utilities|Time|GetWorldDeltaSeconds) (ToolFunction|GetCurveValues "RotationLagSpeed"))))
    (:then_2
      ;[0.15 0.15 0.15 0.5] 平滑根节点
      (Variables|CameraInfo|SetSmoothedPivotTarget (Math|Transform|MakeTransform (ToolFunction|CalculateTransformationTransition (.location (Variables|CameraInfo|GetSmoothedPivotTarget)) (.location (LocalVariables|GetPivotTarget)) (Variables|CameraInfo|GetTargetCameraRotation) (Math|Vector|MakeVector (ToolFunction|GetCurveValues "PivotLagSpeed_X") (ToolFunction|GetCurveValues "PivotLagSpeed_Y") (ToolFunction|GetCurveValues "PivotLagSpeed_Z"))) (.rotation (LocalVariables|GetPivotTarget)))))
    (:then_3
      ;[0.15 0.15 0.15 0.5] 注释
      (Variables|CameraInfo|SetPivotLocation (+ (.location (Variables|CameraInfo|GetSmoothedPivotTarget)) (* (Math|Vector|GetForwardVector (.rotation (Variables|CameraInfo|GetSmoothedPivotTarget))) (ToolFunction|GetCurveValues "PivotOffset_X")) (* (Math|Vector|GetRightVector (.rotation (Variables|CameraInfo|GetSmoothedPivotTarget))) (ToolFunction|GetCurveValues "PivotOffset_Y")) (* (Math|Vector|GetUpVector (.rotation (Variables|CameraInfo|GetSmoothedPivotTarget))) (ToolFunction|GetCurveValues "PivotOffset_Z")))))
    (:then_4
      ;[0.15 0.15 0.15 0.5] 注释
      (Variables|CameraInfo|SetTargetCameraLocation (+ (Variables|CameraInfo|GetPivotLocation) (* (Math|Vector|GetForwardVector (Variables|CameraInfo|GetTargetCameraRotation)) (ToolFunction|GetCurveValues "CameraOffset_X")) (* (Math|Vector|GetRightVector (Variables|CameraInfo|GetTargetCameraRotation)) (ToolFunction|GetCurveValues "CameraOffset_Y")) (* (Math|Vector|GetUpVector (Variables|CameraInfo|GetTargetCameraRotation)) (ToolFunction|GetCurveValues "CameraOffset_Z")))))
    (:then_5
      ;[0.15 0.15 0.15 0.5] 模拟弹簧臂
      (bind (_traceorigin _traceradius _tracechannel) (Class|BPICameraInfo|BPIGet3PTraceParams(Message) (Variables|Default|GetControlledPawn)))
      (bind _outhit (Collision|SphereTraceByChannel _traceorigin (Variables|CameraInfo|GetTargetCameraLocation) _traceradius _tracechannel false 0 "None"))
      (if (and (.bBlockingHit (Collision|BreakHitResult _outhit)) (not (.bInitialOverlap (Collision|BreakHitResult _outhit))))
        (Variables|CameraInfo|SetTargetCameraLocation (+ (- (.Location (Collision|BreakHitResult _outhit)) (.TraceEnd (Collision|BreakHitResult _outhit))) (Variables|CameraInfo|GetTargetCameraLocation)))))
    (:then_6
      ;[0.15 0.15 0.15 0.5] 根据视角返回值
      (return (.location (Math|Transform|Lerp(Transform) (Math|Transform|MakeTransform (Variables|CameraInfo|GetTargetCameraLocation) (Variables|CameraInfo|GetTargetCameraRotation)) (Math|Transform|MakeTransform (LocalVariables|GetFPTarget) (Variables|CameraInfo|GetTargetCameraRotation)) _returnvalue)) (.rotation (Math|Transform|Lerp(Transform) (Math|Transform|MakeTransform (Variables|CameraInfo|GetTargetCameraLocation) (Variables|CameraInfo|GetTargetCameraRotation)) (Math|Transform|MakeTransform (LocalVariables|GetFPTarget) (Variables|CameraInfo|GetTargetCameraRotation)) _returnvalue)) (Math|Float|Lerp (LocalVariables|GetTPFOV) (LocalVariables|GetFPFOV) _returnvalue)))))

(fn GetCurveValues
  (params (CurveName :type Name))
  (bind _cameramesh (Variables|Default|GetCameraMesh))
  (bind _returnvalue (Components|SkeletalMesh|GetAnimInstance _cameramesh))
  (Utilities|IsValid _returnvalue
    (:Is%20Valid
      (return (Animation|Curves|GetCurveValue _returnvalue CurveName)))
    (:Is%20Not%20Valid
      (return 0.0))))

(fn CalculateTransformationTransition
  (params (CurrentLocation :type Vector) (TargetLocation :type Vector) (CameraRotation :type Rotator) (LagSpeeds :type Vector))
  (bind _returnvalue (Utilities|Time|GetWorldDeltaSeconds))
  (LocalVariables|SetCameraRotationYaw (Math|Rotator|MakeRotator 0.0 0.0 (.yaw CameraRotation)))
  (return (Math|Vector|RotateVector (Math|Vector|MakeVector (Math|Interpolation|FInterpTo (.x (Math|Vector|UnrotateVector CurrentLocation (LocalVariables|GetCameraRotationYaw))) (.x (Math|Vector|UnrotateVector TargetLocation (LocalVariables|GetCameraRotationYaw))) _returnvalue (.x LagSpeeds)) (Math|Interpolation|FInterpTo (.y (Math|Vector|UnrotateVector CurrentLocation (LocalVariables|GetCameraRotationYaw))) (.y (Math|Vector|UnrotateVector TargetLocation (LocalVariables|GetCameraRotationYaw))) _returnvalue (.y LagSpeeds)) (Math|Interpolation|FInterpTo (.z (Math|Vector|UnrotateVector CurrentLocation (LocalVariables|GetCameraRotationYaw))) (.z (Math|Vector|UnrotateVector TargetLocation (LocalVariables|GetCameraRotationYaw))) _returnvalue (.z LagSpeeds))) (LocalVariables|GetCameraRotationYaw))))