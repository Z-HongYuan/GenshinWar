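; BP_CopyMesh is a short-lived actor that leaves a frozen mesh copy of its owning GenshinCharacterBase, like an afterimage.
; On BeginPlay it copies the skeletal asset and current pose from the owner's cover mesh onto a PoseableMesh.
; The RenderTime timeline then drives the AlphaControll material parameter, and the actor destroys itself when the timeline finishes.
; It destroys itself immediately if the owner is not that character class.
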(event EventBeginPlay
  (bind _asgenshin_character_base (Utilities|Casting|CastToGenshinCharacterBase (Components|GetOwner))
    (:then
      (Components|SkinnedMesh|SetSkinnedAssetandUpdate (Variables|Default|GetPoseableMesh) (Components|SkeletalMesh|GetSkeletalMeshAsset (Class|GenshinCharacterBase|GetCoverMesh _asgenshin_character_base)) true)
      (Class|PoseableMeshComponent|CopyPosefromSkeletalComponent (Variables|Default|GetPoseableMesh) (Class|GenshinCharacterBase|GetCoverMesh _asgenshin_character_base))
      (bind _render (Timeline|RenderTime PlayFromStart)
        (:Update
          (Rendering|Material|SetScalarParameterValueonMaterials (Variables|Default|GetPoseableMesh) "AlphaControll" _render))
        (:Finished
          (Actor|DestroyActor))))
    (:CastFailed
      (Actor|DestroyActor))))

(fn ConstructionScript)