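; BP_Grenade is a projectile actor that deals an area gameplay effect when its capsule touches anything other than its owner.
; On overlap it runs a multi-sphere object trace for Pawns within RangeRadius at its location, with debug drawing and a printed hit count.
; Each hit actor's Ability System Component applies GE_Test to itself, then the grenade destroys itself.
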(event OnComponentBeginOverlap(CapsuleComponent)
  (params (OverlappedComponent :type Primitive%20Component%20Object%20Reference) (OtherActor :type Actor%20Object%20Reference) (OtherComp :type Primitive%20Component%20Object%20Reference) (OtherBodyIndex :type Integer) (bFromSweep :type Boolean) (SweepResult :type Hit%20Result%20Structure%20%28by%20ref%29))
  (bind _returnvalue (Transformation|GetActorLocation))
  (if (not (== OtherActor (Components|GetOwner)))
    (bind _outhits (Collision|MultiSphereTraceForObjects _returnvalue (+ _returnvalue 0.01) (Variables|Default|GetRangeRadius) (Utilities|Array|MakeArray "ObjectTypeQuery3") false 0 "ForDuration"))
    (Development|PrintString (Utilities|String|ToString(Integer) (Utilities|Array|Length _outhits)))
    (for _array_element _outhits
      (GameplayEffects|ApplyGameplayEffectToSelf (Ability|GetAbilitySystemComponent (.HitActor (Collision|BreakHitResult _array_element))) "/Game/AbilitySystem/Effects/GE_Test.GE_Test_C" 0.0 (GameplayEffects|MakeEffectContext (Ability|GetAbilitySystemComponent (.HitActor (Collision|BreakHitResult _array_element))))))
    (Actor|DestroyActor)))

(event EventBeginPlay)

(event Collision|EventActorBeginOverlap
  (params (OtherActor :type Actor%20Object%20Reference)))

(event EventTick
  (params (DeltaSeconds :type Float%20%28single-precision%29)))

(fn ConstructionScript)